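; Example transition actor that moves the first-person player to the viewpoint of a scene capture camera (CamTransi).
; One second after BeginPlay it disables input, captures the camera's scene and animates a material's Progress parameter over DurationTransi.
; When the timeline finishes, it teleports the character, offset so the eye matches the capture, aligns control rotation, resets Progress and restores input.
; Without a camera set, it prints a warning and destroys itself.
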(event `self.ReceiveBeginPlay`
  ; Setup
  (`TimelineComponent.SetPlayRate` (`self.Transi`) (/ 1.0 (`self.DurationTransi`)))
  (`/Engine/EditorBlueprintResources/StandardMacros.IsValid` (`self.CamTransi`)
    (:`Is Valid`
      (`KismetSystemLibrary.Delay` 1.0)
      (`self.OnTransition`))
    (:`Is Not Valid`
      (`KismetSystemLibrary.PrintString` "No cam setup for transition")
      (`self.K2_DestroyActor`))))

(event `OnTransition`
  (bind _returnvalue (`GameplayStatics.GetPlayerCharacter` 0))
  (bind (_returnvalue_location _returnvalue_rotation) (`KismetMathLibrary.BreakTransform` (`self.GetTransform` (`self.CamTransi`))))
  (`self.DisableInput` (`GameplayStatics.GetPlayerController` 0))
  (`SceneCaptureComponent2D.CaptureScene` (`/Game/Project/Blueprints/BP_CameraTransi.SceneCaptureComponent2D` (`self.CamTransi`)))
  (bind (_direction _float) (`Timeline|Transi` :`NewTime` 5.0 :!via `PlayFromStart`)
    (:`Update`
      (`KismetMaterialLibrary.SetScalarParameterValue` null "Progress" _float))
    (:`Finished`
      (bind _asbp_first_person_character (cast `/Game/FirstPerson/Blueprints/BP_FirstPersonCharacter` _returnvalue))
      (bind _charactermovement (`Character.CharacterMovement` _asbp_first_person_character))
      (`CharacterMovementComponent.DisableMovement` _charactermovement)
      (`self.K2_SetActorLocation` _returnvalue (- _returnvalue_location (.location (`SceneComponent.GetRelativeTransform` (`/Game/FirstPerson/Blueprints/BP_FirstPersonCharacter.FirstPersonCamera` _asbp_first_person_character)))) false false)
      (`CharacterMovementComponent.SetMovementMode` _charactermovement "MOVE_Walking" 0)
      (`Controller.SetControlRotation` (`GameplayStatics.GetPlayerController` 0) _returnvalue_rotation)
      ; Reset du material
      (`KismetMaterialLibrary.SetScalarParameterValue` null "Progress")
      (`self.EnableInput` (`GameplayStatics.GetPlayerController` 0) null))))

(fn `UserConstructionScript`)