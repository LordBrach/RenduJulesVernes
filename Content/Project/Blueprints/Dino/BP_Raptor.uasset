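; Raptor enemy that chases the player across the navmesh and ends the game on catching them.
; From BeginPlay it loops a run animation and re-issues AI MoveTo toward the player every 0.2 seconds.
; Sphere overlap with a BPI_Player actor disables input, blends the camera to the raptor, plays a roar and animation, then only prints the game end.
; Tick prints the movement mode for debugging.
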(event `self.ReceiveBeginPlay`
  (`SkeletalMeshComponent.PlayAnimation` (`self.Mesh`) "/Game/Project/Assets/Dinos/Velociraptor_Anim_Armature_Velociraptor_Run.Velociraptor_Anim_Armature_Velociraptor_Run" true)
  (`self.NavmeshMovePlayer`))

(event `NavmeshMovePlayer`
  (bind _returnvalue (`GameplayStatics.GetPlayerCharacter` 0))
  (`|AIMoveTo` self (`self.K2_GetActorLocation` _returnvalue) _returnvalue 250.0
    (:`then`
      (`KismetSystemLibrary.Delay` 0.2)
      (`self.NavmeshMovePlayer`))
    (:`OnFail`
      (`KismetSystemLibrary.PrintString` "FAIL NAVMESH"))))

(event `StartChase`
  (`self.NavmeshMovePlayer`))

(event `self.Sphere.OnComponentBeginOverlap`
  (params (OverlappedComponent :type "PrimitiveComponent Object Reference") (OtherActor :type "Actor Object Reference") (OtherComp :type "PrimitiveComponent Object Reference") (OtherBodyIndex :type Integer) (bFromSweep :type Boolean) (SweepResult :type "HitResult Structure (by ref)"))
  (bind _returnvalue (`GameplayStatics.GetPlayerController` 0))
  (if (`KismetSystemLibrary.DoesImplementInterface` OtherActor "/Game/Project/Blueprints/BPI_Player.BPI_Player_C")
    (`self.DisableInput` _returnvalue null)
    (`PlayerController.SetViewTargetWithBlend` _returnvalue self 0.5 "VTBlend_Linear" 0.0 false)
    (`SkeletalMeshComponent.PlayAnimation` (`self.Mesh`) "/Game/Project/Assets/Dinos/Velociraptor_Anim_Armature_Velociraptor_Walk.Velociraptor_Anim_Armature_Velociraptor_Walk" false)
    (`GameplayStatics.PlaySoundAtLocation` "/Game/Project/Assets/Sounds/monster_roar.monster_roar" (`SceneComponent.K2_GetComponentLocation` (`self.Mesh`)) (struct) 1.0 1.0 0.0 null null null null)
    (`KismetSystemLibrary.Delay` 1.0)
    (`KismetSystemLibrary.PrintString` "End game")))

(event `self.ReceiveTick`
  (params (DeltaSeconds :type "Float (single-precision)"))
  (`KismetSystemLibrary.PrintString` (`|GetEnumeratorNameAsString` (`CharacterMovementComponent.MovementMode` (`self.CharacterMovement`)))))

(fn `UserConstructionScript`)