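; Interactable elevator button that calls the elevator once, starting disabled until ToggleButton enables it.
; ToggleButton sets usability and swaps between lit and unlit materials, but is ignored once the button has been used.
; The first valid Interact fires CallElevator, plays a blip and unlights the button; later presses only play a randomly low-pitched blip.
; A timeline for the button press animation exists but is never triggered.
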(event `self.ReceiveBeginPlay`
  (set `self.LocationButton` (`SceneComponent.K2_GetComponentLocation` (`self.Button`)))
  (`self.ToggleButton` false))

(event `self.Interact`
  (bind _button (`self.Button`))
  (if (`self.Usable`)
    (if (`self.Used`)
      ; Elevator already called
      (`GameplayStatics.PlaySoundAtLocation` "/Game/Project/Assets/Sounds/blipSelect.blipSelect" (`SceneComponent.K2_GetComponentLocation` (`self.Button`)) (struct) 0.3 (`KismetMathLibrary.RandomFloatInRange` 0.1 0.3) 0.0 null null null null)
      (else
        (set `self.Used` true)
        (`self.CallElevator`)
        (`GameplayStatics.PlaySoundAtLocation` "/Game/Project/Assets/Sounds/blipSelect.blipSelect" (`SceneComponent.K2_GetComponentLocation` _button) (struct) 0.3 1.0 0.0 null null null null)
        (`PrimitiveComponent.SetMaterial` _button 0 "/Game/Project/Levels/Chair.Chair")))))

(event `ToggleButton`
  (params (In :type Boolean))
  (bind _button (`self.Button`))
  (if (not (`self.Used`))
    (bind _output_get (set `self.Usable` In))
    (if _output_get
      (`PrimitiveComponent.SetMaterial` _button 0 "/Game/Project/Assets/Materials/MI_Light.MI_Light")
      (else
        (`PrimitiveComponent.SetMaterial` _button 0 "/Game/Project/Levels/Chair.Chair")))))

(fn `UserConstructionScript`)