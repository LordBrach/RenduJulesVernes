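; Trigger-volume actor that plays a background music track while the player is inside its box.
; On BeginPlay it assigns the BGM sound to its audio component and binds the box's begin and end overlap events.
; Overlaps from actors implementing BPI_Player fade the music in on entry and out on exit.
; An AutoActivate flag also fades the music in at start.
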(event `self.ReceiveBeginPlay`
  (bind _box (`self.Box`))
  (`AudioComponent.SetSound` (`self.Audio`) (`self.BGM`))
  (add `PrimitiveComponent.OnComponentBeginOverlap` _box (delegate `FadeIN`))
  (add `PrimitiveComponent.OnComponentEndOverlap` _box (delegate `FadeOUT`))
  (if (`self.AutoActivate`)
    (`AudioComponent.FadeIn` (`self.Audio`) 1.0 1.0 0.0 "Linear")))

(event `FadeOUT`
  (params (OverlappedComponent :type "PrimitiveComponent Object Reference") (OtherActor :type "Actor Object Reference") (OtherComp :type "PrimitiveComponent Object Reference") (OtherBodyIndex :type Integer))
  (if (`KismetSystemLibrary.DoesImplementInterface` OtherActor "/Game/Project/Blueprints/BPI_Player.BPI_Player_C")
    (`AudioComponent.FadeOut` (`self.Audio`) 1.0 0.0 "Linear")))

(event `FadeIN`
  (params (OverlappedComponent :type "PrimitiveComponent Object Reference") (OtherActor :type "Actor Object Reference") (OtherComp :type "PrimitiveComponent Object Reference") (OtherBodyIndex :type Integer) (bFromSweep :type Boolean) (SweepResult :type "HitResult Structure (by ref)"))
  (if (`KismetSystemLibrary.DoesImplementInterface` OtherActor "/Game/Project/Blueprints/BPI_Player.BPI_Player_C")
    (`AudioComponent.FadeIn` (`self.Audio`) 1.0 1.0 0.0 "Linear")))

(fn `UserConstructionScript`)