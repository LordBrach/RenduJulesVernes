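; BP_DefaultInteractableDialogue is an interactable actor that starts a dialogue when the player interacts with it.
; On Interact it casts the player character to BP_FirstPersonCharacter and calls TryDialogue on its dialogue component with the linked tag and blocking flag.
; A Used flag makes it fire only once unless DoRepeat is set.
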(event `/Game/Project/Blueprints/Interactibles/BPI_Interactible.Interact`
  (if (not (`self.Used`))
    (bind _asbp_first_person_character (cast `/Game/FirstPerson/Blueprints/BP_FirstPersonCharacter` (`GameplayStatics.GetPlayerCharacter` 0)))
    (`/Game/Project/Blueprints/DialogueStuff/ACBP_Dialogue.TryDialogue` (`/Game/FirstPerson/Blueprints/BP_FirstPersonCharacter.ACBP_Dialogue` _asbp_first_person_character) (`self.LinkedTag`) (`self.BlockingDialogue`))
    (if (not (`self.DoRepeat`))
      (set `self.Used` true))))

(fn `UserConstructionScript`)