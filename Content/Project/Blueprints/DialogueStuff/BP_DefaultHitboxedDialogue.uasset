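; A placeable dialogue trigger that starts a tagged dialogue once when the player walks into its linked trigger box.
; On BeginPlay it binds to the linked box's overlap event, or prints a warning naming itself if none is linked.
; When a BPI_Player actor overlaps, it unbinds, calls TryDialogue on the first-person character's dialogue component with its tag and blocking flag, then plays any linked audio.
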(event `self.ReceiveBeginPlay`
  (bind _linkedtriggerbox (`self.LinkedTriggerBox`)
    (:`then`
      (add `self.OnActorBeginOverlap` _linkedtriggerbox (delegate `TriggerEvent`)))
    (:`else`
      (`KismetSystemLibrary.PrintText` (`|FormatText` "No triggerbox linked to {nm}" (`KismetSystemLibrary.GetObjectName` self))))))

(event `TriggerEvent` :!signature `self.OnActorBeginOverlap`
  (params (OverlappedActor :type "Actor Object Reference") (OtherActor :type "Actor Object Reference"))
  (if (`KismetSystemLibrary.DoesImplementInterface` OtherActor "/Game/Project/Blueprints/BPI_Player.BPI_Player_C")
    (remove `self.OnActorBeginOverlap` (`self.LinkedTriggerBox`) (delegate `TriggerEvent`))
    (if (not (`self.Used`))
      (bind _asbp_first_person_character (cast `/Game/FirstPerson/Blueprints/BP_FirstPersonCharacter` (`GameplayStatics.GetPlayerCharacter` 0)))
      (`/Game/Project/Blueprints/DialogueStuff/ACBP_Dialogue.TryDialogue` (`/Game/FirstPerson/Blueprints/BP_FirstPersonCharacter.ACBP_Dialogue` _asbp_first_person_character) (`self.LinkedTag`) (`self.BlockingDialogue`))
      (set `self.Used` true)
      (bind _linkedaudioevent (`self.LinkedAudioEvent`)
        (:`then`
          (`AudioComponent.Play` (`AmbientSound.AudioComponent` _linkedaudioevent) 0.0))
        (:`else`)))))

(fn `UserConstructionScript`)