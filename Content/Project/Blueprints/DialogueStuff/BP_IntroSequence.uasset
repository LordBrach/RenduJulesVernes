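; BP_IntroSequence is an actor that plays a chain of tagged dialogues as an intro when play begins, if enabled.
; It passes the first entry of LinkedTag to the first-person character's dialogue component, with an optional blocking flag.
; When the dialogue widget signals that its text update ended, it removes that tag and plays the next.
; Once the list is empty, it prints a debug message and destroys itself.
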(event `self.ReceiveBeginPlay`
  (if (`self.Enabled`)
    (`self.CallDialogue`)))

(event `CallDialogue`
  (bind _asbp_first_person_character (cast `/Game/FirstPerson/Blueprints/BP_FirstPersonCharacter` (`GameplayStatics.GetPlayerCharacter` 0)))
  (bind _acbp_dialogue (`/Game/FirstPerson/Blueprints/BP_FirstPersonCharacter.ACBP_Dialogue` _asbp_first_person_character))
  (`/Game/Project/Blueprints/DialogueStuff/ACBP_Dialogue.TryDialogue` _acbp_dialogue (`|GetArrayItem` (`self.LinkedTag`)) (`self.BlockingDialogue`))
  (add `/Game/Project/Blueprints/DialogueStuff/WBP_Dialogue.TextUpdateEnded` (`/Game/Project/Blueprints/DialogueStuff/ACBP_Dialogue.WidgetRef` _acbp_dialogue) (delegate `CheckDialogue`)))

(event `CheckDialogue`
  (`KismetArrayLibrary.Array_Remove` (`self.LinkedTag`))
  (if (> (`KismetArrayLibrary.Array_Length` (`self.LinkedTag`)) 0)
    (`self.CallDialogue`)
    (else
      (`KismetSystemLibrary.PrintString` "End Intro")
      (`self.K2_DestroyActor`))))

(fn `UserConstructionScript`)