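; BP_EndingSequence is an ending-sequence actor that spawns dinosaurs when the player enters its linked trigger.
; On BeginPlay it hides its PointLight and binds to the trigger's overlap, unbinding after the first BPI_Player actor enters.
; It spawns one Dino per Spawnpoints entry, all at the player's capsule transform rather than the spawnpoints' transforms.
; After a short delay, it calls NavmeshMovePlayer on each stored Dino.
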(event `self.ReceiveBeginPlay`
  (`self.SetActorHiddenInGame` (`self.PointLight`) true)
  (add `self.OnActorBeginOverlap` (`self.LinkedTrigger`) (delegate `End`)))

(event `End` :!signature `self.OnActorBeginOverlap`
  (params (OverlappedActor :type "Actor Object Reference") (OtherActor :type "Actor Object Reference"))
  (if (`KismetSystemLibrary.DoesImplementInterface` OtherActor "/Game/Project/Blueprints/BPI_Player.BPI_Player_C")
    (remove `self.OnActorBeginOverlap` (`self.LinkedTrigger`) (delegate `End`))
    (for _array_element (`self.Spawnpoints`)
      (bind _returnvalue (`|SpawnActorFromClass` (`self.Dino`) (`SceneComponent.K2_GetComponentToWorld` (`Character.CapsuleComponent` (`GameplayStatics.GetPlayerCharacter` 0))) "AdjustIfPossibleButAlwaysSpawn" "MultiplyWithRoot" null null))
      (`KismetArrayLibrary.Array_AddUnique` (`self.Dinos`) _returnvalue))
    (`KismetSystemLibrary.Delay` 3.0)
    (for _array_element_2 (`self.Dinos`)
      (`/Game/Project/Blueprints/Dino/BP_Raptor.NavmeshMovePlayer` _array_element_2))))

(fn `UserConstructionScript`)